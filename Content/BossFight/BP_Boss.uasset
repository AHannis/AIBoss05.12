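; BP_Boss is a boss character with a melee-style montage attack, an on-screen health bar and ragdoll death.
; A guarded Attack event plays the montage, whose notify fires a long forward sphere trace from ArrowAttack to damage a hit pawn and shakes nearby cameras.
; Incoming damage lowers Health, which Tick pushes to the widget; at zero, movement is disabled and the mesh simulates physics.
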(event `self.ReceiveBeginPlay`
  (bind _returnvalue (`|CreateWidget` "/Game/BossFight/BossHealth.BossHealth_C"))
  (`UserWidget.AddToViewport` _returnvalue 0)
  (set `self.HealthUI` _returnvalue))

(event `self.ReceiveTick`
  (params (DeltaSeconds :type "Float (single-precision)"))
  (`ProgressBar.SetPercent` (`/Game/BossFight/BossHealth.HealthBar` (`self.HealthUI`)) (/ (`self.Health`) 100.0)))

(event `/Game/BossFight/BP_BossFight.Attack`
  (bind _arrowattack (`self.ArrowAttack`))
  (bind _returnvalue (`SceneComponent.K2_GetComponentLocation` _arrowattack))
  ; Attack
  (if (not (`self.isAttacking?`))
    (`|PlayMontage` (`self.Mesh`) "/Game/BossCharacter/Fight2_Montage.Fight2_Montage"
      (:`then`
        (set `self.isAttacking?` true))
      (:`OnCompleted`
        (set `self.isAttacking?` false))
      (:`OnNotifyBegin`
        (`|ExecutionSequence`
          (:`then_0`
            (bind (_outhit _returnvalue_2) (`KismetSystemLibrary.SphereTraceSingleForObjects` :`Start` _returnvalue :`End` (+ _returnvalue (* (`KismetMathLibrary.GetForwardVector` (`SceneComponent.K2_GetComponentRotation` _arrowattack)) 3000.0)) :`Radius` 35.0 :`ObjectTypes` (`|MakeArray` "ObjectTypeQuery3" :!type "EObjectTypeQuery Enum") :`DrawDebugType` "ForDuration" :`DrawTime` 2.0))
            (if _returnvalue_2
              (`GameplayStatics.ApplyDamage` (`.HitActor` (`GameplayStatics.BreakHitResult` _outhit)) 10.0)))
          (:`then_1`
            (`GameplayStatics.PlayWorldCameraShake` "/Game/BossFight/Attack_CameraShake.Attack_CameraShake_C" (`self.K2_GetActorLocation`) 0.0 3500.0)))))))

(event `self.ReceiveAnyDamage`
  (params (Damage :type "Float (single-precision)") (DamageType :type "DamageType Object Reference") (InstigatedBy :type "Controller Object Reference") (DamageCauser :type "Actor Object Reference"))
  ; Health
  (set `self.Health` (- (`self.Health`) Damage))
  (if (<= (`self.Health`) 0.0)
    (`CharacterMovementComponent.DisableMovement` (`self.CharacterMovement`))
    (`PrimitiveComponent.SetSimulatePhysics` (`self.Mesh`) true)))

(fn `UserConstructionScript`)